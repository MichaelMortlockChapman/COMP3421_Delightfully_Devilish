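; Kitchen fridge door that toggles open and closed on left click while the player's box component overlaps its trigger box.
; It binds to Player_BP's click event and swings the mesh with a timeline after a short delay.
; Opening spawns fresh chicken, carrot, potato and herbs and teleports them onto shelves.
; Closing reverses the swing, then destroys any Item_BP actors inside the deletion box.
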(event OnComponentBeginOverlap(Box)
  (params (OverlappedComponent :type Primitive%20Component%20Object%20Reference) (OtherActor :type Actor%20Object%20Reference) (OtherComp :type Primitive%20Component%20Object%20Reference) (OtherBodyIndex :type Integer) (bFromSweep :type Boolean) (SweepResult :type Hit%20Result%20Structure%20%28by%20ref%29))
  ;[1 1 1] Set LookingAt Var
  (if (== (Actor|GetComponentbyClass (stale EventBeginPlay _asplayer_bp) "/Script/Engine.BoxComponent") OtherComp)
    (Variables|Default|SetLookingAt true)))

(event OnComponentEndOverlap(Box)
  (params (OverlappedComponent :type Primitive%20Component%20Object%20Reference) (OtherActor :type Actor%20Object%20Reference) (OtherComp :type Primitive%20Component%20Object%20Reference) (OtherBodyIndex :type Integer))
  ;[1 1 1] Set LookingAt Var
  (if (== (Actor|GetComponentbyClass (stale EventBeginPlay _asplayer_bp) "/Script/Engine.BoxComponent") OtherComp)
    (Variables|Default|SetLookingAt false)))

(event Custom|OnLMB
  (bind _deletionbox (Variables|Default|GetDeletionBox))
  ;[1 1 1] Get LMB Input
  (if (Variables|Default|GetLookingAt)
    (Utilities|FlowControl|Sequence
      (:then_0
        (if (not (Variables|Default|GetOpened))
          (Utilities|FlowControl|Sequence
            (:then_0
              (|SpawnItems))
            (:then_1
              ;[1 1 1] Play Door Animation
              (Utilities|FlowControl|Delay 0.8)
              (bind _newtrack_0 (Timeline|Timeline Play)
                (:Update
                  (Transformation|SetRelativeRotation (Variables|Default|GetStaticMesh) (Math|Rotator|MakeRotator 0.0 0.0 _newtrack_0) false false)))))
          (else
            (Utilities|FlowControl|Delay 0.8)
            (Utilities|FlowControl|Sequence
              (:then_0
                (Timeline|Timeline ReverseFromEnd))
              (:then_1
                ;[1 1 1] Delete Fridge Contents
                (Utilities|FlowControl|Delay 1.0)
                (bind _outactors (Collision|ComponentOverlapActors _deletionbox (Transformation|GetWorldTransform _deletionbox) (Utilities|Array|MakeArray "ObjectTypeQuery2") "/Game/Dynamic/Food/item_BP.item_BP_C"))
                (for _array_element _outactors
                  (Actor|DestroyActor _array_element)))))))
      (:then_1
        (Variables|Default|SetOpened (not (Variables|Default|GetOpened)))))))

(event EventBeginPlay
  ;[1 1 1] Get LMB Input
  (bind _asplayer_bp (Utilities|Casting|CastToPlayer_BP (Game|GetPlayerCharacter 0)))
  (EventDispatchers|BindEventtoLMBPress _asplayer_bp (delegate Custom|OnLMB)))

(fn ConstructionScript)