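; Food item actor whose mesh changes when the correct piece of equipment is used on it.
; SettingClassVars stores the replacement mesh, the accepted equipment name and left and right finger socket names.
; Modify records the equipment and, after a short delay, calls ChangeItem, which on a name match nudges the mesh upward, swaps it and flags the item as modified.
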(event Custom|Modify
  (params (equip :type String))
  (Variables|Default|SetEquip equip)
  (Utilities|FlowControl|Delay 0.8)
  (CallFunction|ChangeItem (Variables|Default|GetitemName) (Variables|Default|GetInteractableEquipName) (Variables|Default|GetNewItemMesh)))

(event Custom|SettingClassVars
  (params (NewItemMesh_ :type Static%20Mesh%20Object%20Reference) (InteractableEquipName_ :type String))
  (Variables|Default|SetNewItemMesh NewItemMesh_)
  (Variables|Default|SetInteractableEquipName InteractableEquipName_)
  (Variables|Default|SetRightSocket "R_fingersSocket")
  (Variables|Default|SetLeftSocket "L_fingersSocket"))

(event Collision|EventActorBeginOverlap
  (params (OtherActor :type Actor%20Object%20Reference)))

(event EventTick
  (params (DeltaSeconds :type Float%20%28single-precision%29)))

(fn ConstructionScript)

(fn ChangeItem
  (params (ItemString :type String) (EquipString :type String) (NewMesh :type Static%20Mesh%20Object%20Reference))
  (bind _itemmesh (Variables|Default|GetitemMesh))
  (bind _returnvalue (Transformation|GetWorldLocation _itemmesh))
  ;[1 1 1] Equipment Function
  ;;[1 1 1] Move Mesh Up
  (if (and (Utilities|Enum|Equal(Enum) (Variables|Default|GetitemName) ItemString) (Utilities|Enum|Equal(Enum) (Variables|Default|GetEquip) EquipString))
    (Transformation|SetWorldLocation _itemmesh (Math|Vector|MakeVector (.x _returnvalue) (.y _returnvalue) (+ (.z _returnvalue) 2e+01)) false true)
    (Components|StaticMesh|SetStaticMesh _itemmesh NewMesh)
    (Variables|Default|SetisModified true)))