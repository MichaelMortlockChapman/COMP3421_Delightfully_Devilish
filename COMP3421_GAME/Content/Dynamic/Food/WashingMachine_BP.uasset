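; Food prop Blueprint for a washing machine that works as a blender, combining dropped carrot, potato, tomato sauce and a knife.
; Overlapping unheld item_BP actors run through chained name checks, which destroy the match, flag it and show that ingredient's mesh.
; UnequipInteract nudges the machine upward and, once a knife is added, sets IsBlended.
; The combined mesh then replaces ingredients if potato and tomato are present; CarrotAdded is never checked.
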(event OnComponentBeginOverlap(WashingMachine)
  (params (OverlappedComponent :type Primitive%20Component%20Object%20Reference) (OtherActor :type Actor%20Object%20Reference) (OtherComp :type Primitive%20Component%20Object%20Reference) (OtherBodyIndex :type Integer) (bFromSweep :type Boolean) (SweepResult :type Hit%20Result%20Structure%20%28by%20ref%29))
  (bind _asitem_bp (Utilities|Casting|CastToitem_BP OtherActor))
  (bind _output_get (Variables|Default|SetincomingItem _asitem_bp))
  (if (not (Variables|/Game/Dynamic/Food/item_BP.item_BP_C|GetisBeingHeld _output_get))
    (|addCarrot
      (:false
        (|addPotato
          (:false
            (|addTomato
              (:false
                (|addKnife)))))))))

(event EventBeginPlay)

(event Collision|EventActorBeginOverlap
  (params (OtherActor :type Actor%20Object%20Reference)))

(event EventTick
  (params (DeltaSeconds :type Float%20%28single-precision%29)))

(event EventUnequipInteract
  (bind _washingmachine (Variables|Default|GetWashingMachine))
  (bind _returnvalue (Transformation|GetWorldLocation _washingmachine))
  (Transformation|SetWorldLocation _washingmachine (Math|Vector|MakeVector (.x _returnvalue) (.y _returnvalue) (+ (.z _returnvalue) 1e+01)) false false)
  (if (Variables|Default|Getknife_added)
    (Variables|Default|SetisBlended true)
    (if (Math|Boolean|ANDBoolean (Variables|Default|Getpotato_added) (Variables|Default|Gettomato_added) (Variables|Default|Getpotato_added) (Variables|Default|Getknife_added))
      (Rendering|SetVisibility (Variables|Default|GetCarrot) false false)
      (Rendering|SetVisibility (Variables|Default|GetTomato) false false)
      (Rendering|SetVisibility (Variables|Default|GetPotato) false false)
      (Rendering|SetVisibility (Variables|Default|GetCombined) true false))))

(fn ConstructionScript)

(fn GetDishStruc)