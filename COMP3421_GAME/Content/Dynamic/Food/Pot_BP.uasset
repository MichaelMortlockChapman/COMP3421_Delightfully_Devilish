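; Soup pot that collects ingredient items dropped into it and records what the dish contains.
; On overlap with an item_BP not being held, chained macros match its name, reveal that soup component, destroy the item and set a flag.
; GetDishStruc returns those flags as an ingredient map of 1/0 values.
; Spice also triggers, via FlipFlop on alternate additions, a devil level sequence, briefly disabling player input before spawning an actor.
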(event OnComponentBeginOverlap(soup_pot)
  (params (OverlappedComponent :type Primitive%20Component%20Object%20Reference) (OtherActor :type Actor%20Object%20Reference) (OtherComp :type Primitive%20Component%20Object%20Reference) (OtherBodyIndex :type Integer) (bFromSweep :type Boolean) (SweepResult :type Hit%20Result%20Structure%20%28by%20ref%29))
  (bind _asitem_bp (Utilities|Casting|CastToitem_BP OtherActor))
  (bind _output_get (Variables|Default|SetincomingItem _asitem_bp))
  (if (not (Variables|/Game/Dynamic/Food/item_BP.item_BP_C|GetisBeingHeld _output_get))
    (|addCarrot
      (:false
        (|addPotato
          (:false
            (|addHerb
              (:false
                (|addChicken
                  (:false
                    (|addSpice)))))))))))

(event Custom|add%20stuff
  (params (Ingredient :type String)))

(event Custom|SpawnDevilEvent
  (bind _returnvalue (Game|Player|GetPlayerPawn 0))
  (bind _returnvalue_2 (Game|GetPlayerController 0))
  ;[1 1 1] Seqence (SpawnDevil) logic
  (Input|DisableInput _returnvalue _returnvalue_2)
  (Utilities|FlowControl|Delay 2.9)
  (Input|EnableInput _returnvalue _returnvalue_2)
  (Game|SpawnActorfromClass "/Game/Dynamic/Devil/Devil_BP.Devil_BP_C" (Math|Transform|MakeTransform "10.000000,-260.000000,60.000000" "0, 0, 0" "1.000000,1.000000,1.000000") "Undefined" "MultiplyWithRoot" 0 0) ; Spawning rather than using keep state in level sequence as latter not working for me
)

(event EventBeginPlay)

(event Collision|EventActorBeginOverlap
  (params (OtherActor :type Actor%20Object%20Reference)))

(event EventTick
  (params (DeltaSeconds :type Float%20%28single-precision%29)))

(fn ConstructionScript)

(fn GetDishStruc
  (return (Utilities|Struct|MakeDish_Struc (Utilities|Map|MakeMap "chicken" (Math|Conversions|ToFloat(Integer) (Math|Integer|SelectInt 1 0 (Variables|Default|Getchicken_added))) "spice" (Math|Conversions|ToFloat(Integer) (Math|Integer|SelectInt 1 0 (Variables|Default|Getspice_added))) "potato" (Math|Conversions|ToFloat(Integer) (Math|Integer|SelectInt 1 0 (Variables|Default|Getpotato_added))) "carrot" (Math|Conversions|ToFloat(Integer) (Math|Integer|SelectInt 1 0 (Variables|Default|Getcarrot_added))) "basil" (Math|Conversions|ToFloat(Integer) (Math|Integer|SelectInt 1 0 (Variables|Default|Getbasil_added)))))))