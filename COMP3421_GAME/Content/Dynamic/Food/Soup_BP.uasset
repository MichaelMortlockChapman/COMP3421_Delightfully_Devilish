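; Soup pot Blueprint that collects dropped food ingredients and shows them as soup contents.
; When an item_BP that is not being held overlaps the pot, a chain of macros checks its name against carrot, potato, herb, chicken and spice.
; A match reveals the corresponding soup component (spice reveals the broth) and destroys the item.
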(event OnComponentBeginOverlap(soup_pot)
  (params (OverlappedComponent :type Primitive%20Component%20Object%20Reference) (OtherActor :type Actor%20Object%20Reference) (OtherComp :type Primitive%20Component%20Object%20Reference) (OtherBodyIndex :type Integer) (bFromSweep :type Boolean) (SweepResult :type Hit%20Result%20Structure%20%28by%20ref%29))
  (bind _asitem_bp (Utilities|Casting|CastToitem_BP OtherActor))
  (bind _output_get (Variables|Default|SetincomingItem _asitem_bp))
  (if (not (Variables|/Game/Dynamic/Food/item_BP.item_BP_C|GetisBeingHeld _output_get))
    (|addCarrot
      (:false
        (|addPotato
          (:false
            (|addHerb
              (:false
                (|addChicken
                  (:false
                    (|addSpice)))))))))))

(event Custom|add%20stuff
  (params (Ingredient :type String)))

(event EventBeginPlay)

(event Collision|EventActorBeginOverlap
  (params (OtherActor :type Actor%20Object%20Reference)))

(event EventTick
  (params (DeltaSeconds :type Float%20%28single-precision%29)))

(fn ConstructionScript)