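; Devil character Blueprint that reacts to the player's proximity, wins and losses, and takes submitted dishes.
; Tick checks the player's distance and sets PlayerNear on Devil_Anim_BP unless the game is already won or lost; win and lose events set matching animation flags.
; Submitted items snap to the devil's right-hand finger socket.
; A capture event hides the player, renders a SceneCapture2D and exports it as a PNG to the project's Photos folder.
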(event Custom|Capture%20Scene%20Event
  (bind _scenecapturecomponent2d (Variables|Default|GetSceneCaptureComponent2D))
  ;[1 1 1] Capture
  ;;[1 1 1] Hide Player
  (bind _returnvalue (Actor|GetActorOfClass "/Game/Dynamic/Player/Player_BP.Player_BP_C"))
  (Class|SceneCaptureComponent|HideActorComponents (Variables|Default|GetSceneCaptureComponent2D) _returnvalue true)
  (Utilities|FlowControl|Delay 0.2)
  (Rendering|SceneCapture|CaptureScene _scenecapturecomponent2d :!class /Script/Engine.SceneCaptureComponent2D)
  (Rendering|ExportRenderTarget (Variables|/Script/Engine.SceneCaptureComponent2D|GetTextureTarget _scenecapturecomponent2d) (Utilities|String|Append (Class|KismetSystemLibrary|GetProjectDirectory) "/Photos/") "capture.png")
  (Development|PrintString "Saved Photo"))

(event Custom|WinEvent
  ;[1 1 1] Player Win
  (bind _devilanimbp (Utilities|GetDevilAnimBP)
    (:End
      (Variables|/Game/Dynamic/Devil/Devil_Anim_BP.Devil_Anim_BP_C|SetPlayerWin _devilanimbp true))))

(event Custom|AttachItemEvent
  (params (ItemObj :type Item%20BP%20Object%20Reference))
  ;[1 1 1] Attach Submitted Dish
  (Transformation|AttachComponentToComponent ItemObj (Variables|Default|Getdevil_mesh) "R_fingersSocket" "SnapToTarget" "SnapToTarget" "SnapToTarget" true))

(event Custom|LoseEvent
  ;[1 1 1] Player Lose
  (bind _devilanimbp (Utilities|GetDevilAnimBP)
    (:End
      (Variables|/Game/Dynamic/Devil/Devil_Anim_BP.Devil_Anim_BP_C|SetPlayerLose _devilanimbp true))))

(event EventTick
  (params (DeltaSeconds :type Float%20%28single-precision%29))
  ;[1 1 1] Near Player
  (bind _outactors (Actor|GetAllActorsOfClass "/Game/Dynamic/Player/Player_BP.Player_BP_C"))
  (bind _devilanimbp (Utilities|GetDevilAnimBP)
    (:End
      (Variables|/Game/Dynamic/Devil/Devil_Anim_BP.Devil_Anim_BP_C|SetPlayerNear _devilanimbp (and (and (not (Variables|/Game/Dynamic/Devil/Devil_Anim_BP.Devil_Anim_BP_C|GetPlayerWin _devilanimbp)) (not (Variables|/Game/Dynamic/Devil/Devil_Anim_BP.Devil_Anim_BP_C|GetPlayerLose _devilanimbp))) (CallFunction|NearDevil (Utilities|Array|Get(acopy) _outactors)))))))

(fn ConstructionScript)

(fn NearDevil
  (params (NewParam :type Player%20BP%20Object%20Reference))
  (return (<= (Transformation|GetDistanceTo NewParam) (Variables|Default|GetNearConstant))))