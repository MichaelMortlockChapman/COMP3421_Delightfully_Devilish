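; Level system Blueprint that judges a submitted dish to win or lose the level and applies saved sound volumes through a sound mix.
; Submit_Dish totals ingredient ratings weighted by DishConstants and compares the result to DemonAcceptanceConstant.
; Win or lose triggers the Devil's event and saves level completion flags or the current level to slot 1.
; It then hides the player from the Devil's scene capture, disables input and shows the end menu.
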(event Custom|Submit_Dish
  (params (Dish :type Dish%20Struc%20Structure))
  ;[1 1 1] Level End System
  ;;[1 1 1] Win/Lose System
  (bind _keys (Utilities|Map|Keys (.dish_ingredient_map Dish)))
  (for _array_element _keys
    (Utilities|UpdateFinalDishValue _array_element (.Value (Utilities|Map|Find (.dish_ingredient_map Dish) _array_element))))
  (if (>= (Variables|Default|GetFinalDishValue) (Variables|Default|GetDemonAcceptanceConstant))
    (CallFunction|WinLevel)
    (else
      (CallFunction|LoseLevel)))
  (Utilities|HidePlayerfromCapture)
  (Utilities|TogglePlayerInput false
    (:End
      (Utilities|FlowControl|Delay 0.0)
      ;;[1 1 1] End Menu GUI
      (bind _asplayer_bp (Utilities|Casting|CastToPlayer_BP (Game|Player|GetPlayerPawn 0)))
      (Default|RemoveHUDEvent _asplayer_bp)
      (bind _returnvalue (UserInterface|CreateWidget "/Game/Dynamic/System/GUI/End_Menu_Widget_BP.End_Menu_Widget_BP_C"))
      (UserInterface|Viewport|AddtoViewport _returnvalue 0)
      (Variables|/Script/Engine.PlayerController|SetbShowMouseCursor (Game|GetPlayerController 0) true))))

(event Custom|StartSoundMixEvent
  ;[1 1 1] On construct Load and Set sliders to volume
  (Class|GameplayStatics|SetBaseSoundMix "/Game/Static/Sounds/SFX_Mix.SFX_Mix")
  (bind _returnvalue (SaveGame|DoesSaveGameExist "2"))
  (if _returnvalue
    (bind _returnvalue_2 (SaveGame|LoadGamefromSlot "2"))
    (bind _assave_system_bp (Utilities|Casting|CastToSave_system_BP _returnvalue_2))
    (for (_array_element _array_index) (Variables|/Game/Dynamic/System/Save_system_BP.Save_system_BP_C|GetsoundVolumes _assave_system_bp)
      (switch int _array_index
        (:0
          (Audio|SetSoundMixClassOverride "/Game/Static/Sounds/SFX_Mix.SFX_Mix" "/Game/Static/Sounds/SFX_Music.SFX_Music" _array_element 1.0 0.0 true))
        (:1
          (Audio|SetSoundMixClassOverride "/Game/Static/Sounds/SFX_Mix.SFX_Mix" "/Game/Static/Sounds/SFX_Effects.SFX_Effects" _array_element 1.0 0.0 true))))))

(fn ConstructionScript)

(fn WinLevel
  (Development|PrintString "Win")
  (bind _outactors (Actor|GetAllActorsOfClass "/Game/Dynamic/Devil/Devil_BP.Devil_BP_C"))
  (Default|WinEvent (Utilities|Array|Get(acopy) _outactors))
  (Variables|Default|SetLevelComplete true)
  ;[1 1 1] Save game exists
  (bind _returnvalue (SaveGame|LoadGamefromSlot "1"))
  (bind _assave_system_bp (Utilities|Casting|CastToSave_system_BP _returnvalue))
  (bind _returnvalue_2 (Game|GetCurrentLevelName true))
  (switch string _returnvalue_2
    (:Kitchen_START
      (Variables|/Game/Dynamic/System/Save_system_BP.Save_system_BP_C|SettutorialDone? _assave_system_bp true))
    (:BathroomMap
      (Variables|/Game/Dynamic/System/Save_system_BP.Save_system_BP_C|SetbathroomDone? _assave_system_bp true))
    (:Garage
      (Variables|/Game/Dynamic/System/Save_system_BP.Save_system_BP_C|SetgarageDone? _assave_system_bp true)))
  (SaveGame|SaveGametoSlot _assave_system_bp "1"))

(fn LoseLevel
  (Development|PrintString "Lose")
  (bind _outactors (Actor|GetAllActorsOfClass "/Game/Dynamic/Devil/Devil_BP.Devil_BP_C"))
  (Default|LoseEvent (Utilities|Array|Get(acopy) _outactors))
  (Variables|Default|SetLevelComplete false)
  ;[1 1 1] Save game system
  (bind _returnvalue (SaveGame|DoesSaveGameExist "1"))
  (if _returnvalue
    ;;[1 1 1] Save game exists
    (bind _returnvalue_2 (SaveGame|LoadGamefromSlot "1"))
    (bind _assave_system_bp (Utilities|Casting|CastToSave_system_BP _returnvalue_2))
    (bind _returnvalue_3 (Game|GetCurrentLevelName true))
    (Variables|/Game/Dynamic/System/Save_system_BP.Save_system_BP_C|SetcurrentLevel _assave_system_bp (Utilities|String|StringToName _returnvalue_3))
    (SaveGame|SaveGametoSlot _assave_system_bp "1")))