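; First-person player Blueprint for a cooking game, with independently controlled left and right hands.
; Mouse buttons run delayed grab/drop on overlapping items using arm sockets and physics toggles, while E/Q modify items, fill plates or use food containers.
; Middle mouse submits the left-hand dish to the level system near the Devil, switching cameras.
; It also handles Enhanced Input movement, HUD, interface interactions, photo selection and trace-to-UV whiteboard drawing.
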(event Custom|RemoveHUDEvent
  ;[1 1 1] Remove HUD event
  (bind _foundwidgets (Widget|GetAllWidgetsOfClass "/Game/Dynamic/System/GUI/HUD_Widget_BP.HUD_Widget_BP_C" true))
  (Widget|RemovefromParent (Utilities|Array|Get(acopy) _foundwidgets)))

(event Custom|AddHUDEvent
  ;[1 1 1] Create/Add HUD
  (bind _returnvalue (UserInterface|CreateWidget "/Game/Dynamic/System/GUI/HUD_Widget_BP.HUD_Widget_BP_C"))
  (UserInterface|Viewport|AddtoViewport _returnvalue 0))

(event Input|EnhancedActionEvents|EnhancedInputActionIA_look
  (params (ActionValue :type Vector%202D%20Structure) (ElapsedSeconds :type Float%20%28double-precision%29) (TriggeredSeconds :type Float%20%28double-precision%29) (InputAction :type Input%20Action%20Object%20Reference :default "/Game/Dynamic/Player/IA_look.IA_look"))
  ;[1 1 1] Camera
  (Pawn|Input|AddControllerYawInput (.x ActionValue))
  (Pawn|Input|AddControllerPitchInput (* (.y ActionValue) -1.0)))

(event Input|EnhancedActionEvents|EnhancedInputActionIA_move
  (params (ActionValue :type Vector%202D%20Structure) (ElapsedSeconds :type Float%20%28double-precision%29) (TriggeredSeconds :type Float%20%28double-precision%29) (InputAction :type Input%20Action%20Object%20Reference :default "/Game/Dynamic/Player/IA_move.IA_move"))
  (bind _returnvalue (Pawn|GetControlRotation :!class /Script/Engine.Pawn))
  (bind _returnvalue_2 (Pawn|GetControlRotation :!class /Script/Engine.Pawn))
  ;[1 1 1] Movement
  (Pawn|Input|AddMovementInput (Math|Vector|GetRightVector (Math|Rotator|MakeRotator (.roll _returnvalue) 0.0 (.yaw _returnvalue))) (.x ActionValue) false)
  (Pawn|Input|AddMovementInput (Math|Vector|GetForwardVector (Math|Rotator|MakeRotator (.roll _returnvalue_2) 0.0 (.yaw _returnvalue_2))) (.y ActionValue) false))

(event Input|EnhancedActionEvents|EnhancedInputActionIA_leftArmAction
  (params (ActionValue :type Boolean) (ElapsedSeconds :type Float%20%28double-precision%29) (TriggeredSeconds :type Float%20%28double-precision%29) (InputAction :type Input%20Action%20Object%20Reference :default "/Game/Dynamic/Player/IA_leftArmAction.IA_leftArmAction"))
  (Components|Animation|PlayAnimation (Variables|Components|Getarms) "/Game/Static/Assets/Player/arms_left_action.arms_left_action" false)
  (Input|DisableInput 0)
  (Utilities|FlowControl|Delay 0.8)
  (Input|EnableInput 0))

(event Input|EnhancedActionEvents|EnhancedInputActionIA_rightArmAction
  (params (ActionValue :type Boolean) (ElapsedSeconds :type Float%20%28double-precision%29) (TriggeredSeconds :type Float%20%28double-precision%29) (InputAction :type Input%20Action%20Object%20Reference :default "/Game/Dynamic/Player/IA_rightArmAction.IA_rightArmAction"))
  (Components|Animation|PlayAnimation (Variables|Components|Getarms) "/Game/Static/Assets/Player/arms_right_action.arms_right_action" false)
  (Input|DisableInput 0)
  (Utilities|FlowControl|Delay 0.8)
  (Input|EnableInput 0))

(event EventBeginPlay
  ;[1 1 1] On Start
  (CallFunction|AddHUDEvent)
  ;[1 1 1] Input Mapping
  (bind _asplayer_controller (Utilities|Casting|CastToPlayerController (Pawn|GetController)))
  (Utilities|IsValid (PlayerController|LocalPlayerSubsystems|GetEnhancedInputLocalPlayerSubsystem _asplayer_controller)
    (:Is%20Valid
      (Input|AddMappingContext (PlayerController|LocalPlayerSubsystems|GetEnhancedInputLocalPlayerSubsystem _asplayer_controller) "/Game/Dynamic/Player/IMC_Player.IMC_Player" 0 "(bIgnoreAllPressedKeysUntilRelease=True,bForceImmediately=False,bNotifyUserSettings=False)"))))

(event EventTick
  (params (DeltaSeconds :type Float%20%28single-precision%29))
  (bind _camera (Variables|Components|GetCamera))
  (bind _returnvalue (Transformation|GetWorldLocation _camera))
  (if (Variables|Default|GetIsDrawing)
    (bind (_outhit _returnvalue_2) (Collision|LineTraceByChannel _returnvalue (+ (* (Math|Vector|GetForwardVector _camera) 1e+03) _returnvalue) "TraceTypeQuery1" false 0 "None"))
    (if _returnvalue_2
      (bind _aswhiteboard_actor (Utilities|Casting|CastToWhiteboard_Actor (.HitActor (Collision|BreakHitResult _outhit))))
      (Default|DrawonWhiteboard _aswhiteboard_actor (.UV (Class|GameplayStatics|FindCollisionUV _outhit))))))

(event Input|ActionEvents|InputActionInteract
  (params (Key :type Key%20Structure :default "None"))
  ;[1 1 1] Interact with doors
  (:Pressed
    (bind _array_element (Utilities|Array|ForEachLoopwithBreak (Collision|GetOverlappingActors 0 :!class /Script/Engine.Actor) :!label _label)
      (:LoopBody
        (if (Utilities|DoesObjectImplementInterface _array_element "/Game/Dynamic/Interfaces/InteractInterface.InteractInterface_C")
          (Class|InteractInterface|Interact(Message) _array_element)
          (goto _label Break))))))

(event Input|MouseEvents|MiddleMouseButton
  (params (Key :type Key%20Structure :default "None"))
  (bind _leftitem (Variables|Default|GetleftItem))
  ;[1 1 1] Dish Submitting
  (:Released
    (bind _outactors (Actor|GetAllActorsOfClass "/Game/Dynamic/Devil/Devil_BP.Devil_BP_C"))
    (bind _asdevil_bp (Utilities|Casting|CastToDevil_BP (Utilities|Array|Get(acopy) _outactors)))
    (if (Default|NearDevil _asdevil_bp self)
      (Default|AttachItemEvent _asdevil_bp _leftitem)
      (bind _asplating_bp (Utilities|Casting|CastToplating_BP _leftitem)
        (:then
          ;;[1 1 1] Left item is Plating BP
          (Variables|Default|SetDish (Variables|/Game/Dynamic/Food/plating_BP.plating_BP_C|GetdishStruc _asplating_bp)))
        (:CastFailed
          ;;[1 1 1] Left item is not Plating BP
          (Variables|Default|SetDish (Utilities|Struct|MakeDish_Struc (Utilities|Map|MakeMap "None" 0.0)))))
      (bind _returnvalue (Actor|GetActorOfClass "/Game/Dynamic/System/Level_system_BP.Level_system_BP_C"))
      ;[1 1 1] TESTING #REMOVE
      (bind _keys (Utilities|Map|Keys (.dish_ingredient_map (Variables|Default|GetDish))))
      (for _array_element _keys
        (Development|PrintText (Utilities|Text|FormatText "{1}: {2}" _array_element (.Value (Utilities|Map|Find (.dish_ingredient_map (Variables|Default|GetDish)) _array_element)))))
      (Default|SubmitDish _returnvalue (Utilities|Struct|MakeDish_Struc (.dish_ingredient_map (Variables|Default|GetDish))))
      (bind _returnvalue_2 (Actor|GetActorOfClass "/Game/Dynamic/Devil/Devil_BP.Devil_BP_C"))
      (Components|Activation|SetActive (Components|GetChildComponent (Variables|/Game/Dynamic/Devil/Devil_BP.Devil_BP_C|GetCameraSceneCapture _returnvalue_2) 0) true false)
      (Components|Activation|SetActive (Variables|Components|GetCamera) false false))))

(event Input|KeyboardEvents|SpaceBar
  (params (Key :type Key%20Structure :default "None"))
  (:Pressed
    (Variables|Default|SetIsDrawing true))
  (:Released
    (Variables|Default|SetIsDrawing false)))

(event Input|KeyboardEvents|E
  (params (Key :type Key%20Structure :default "None"))
  (:Pressed
    (if (Variables|Default|GetrightEquip)
      (for _array_element (Collision|GetOverlappingActors (Variables|Default|GetpickUpBox) "/Game/Dynamic/Food/item_BP.item_BP_C" :!class /Script/Engine.PrimitiveComponent)
        (bind _asitem_bp (Utilities|Casting|CastToitem_BP _array_element))
        (Default|Modify _asitem_bp (Variables|/Game/Dynamic/Food/item_BP.item_BP_C|GetitemName (Variables|Default|GetrightItem)))
        (Development|PrintString "mod")))))

(event Input|KeyboardEvents|E
  (params (Key :type Key%20Structure :default "None"))
  (bind _pickupbox (Variables|Default|GetpickUpBox))
  (:Pressed
    (Utilities|FlowControl|Delay 0.8)
    (if (Variables|Default|GetrightEquip)
      (for _array_element (Collision|GetOverlappingActors _pickupbox "/Game/Dynamic/Food/foodContainer_BP.foodContainer_BP_C" :!class /Script/Engine.PrimitiveComponent)
        (bind _asfood_container_bp (Utilities|Casting|CastTofoodContainer_BP _array_element))
        (bind _asplating_bp (Utilities|Casting|CastToplating_BP (Variables|Default|GetrightItem)))
        (Default|Fill _asplating_bp _asfood_container_bp))
      (else
        (for _array_element_2 (Collision|GetOverlappingActors _pickupbox "/Game/Dynamic/Food/foodContainer_BP.foodContainer_BP_C" :!class /Script/Engine.PrimitiveComponent)
          (bind _asfood_container_bp_2 (Utilities|Casting|CastTofoodContainer_BP _array_element_2))
          (Default|UnequipInteract _asfood_container_bp_2))))))

(event Input|KeyboardEvents|Q
  (params (Key :type Key%20Structure :default "None"))
  (:Pressed
    (if (Variables|Default|GetleftEquip)
      (for _array_element (Collision|GetOverlappingActors (Variables|Default|GetpickUpBox) "/Game/Dynamic/Food/item_BP.item_BP_C" :!class /Script/Engine.PrimitiveComponent)
        (bind _asitem_bp (Utilities|Casting|CastToitem_BP _array_element))
        (Default|Modify _asitem_bp (Variables|/Game/Dynamic/Food/item_BP.item_BP_C|GetitemName (Variables|Default|GetleftItem)))
        (Development|PrintString "mod")))))

(event Input|MouseEvents|LeftMouseButton
  (params (Key :type Key%20Structure :default "None"))
  (:Pressed
    (Utilities|FlowControl|Delay 0.8)
    (|leftGrab)
    (|leftDrop)))

(event Input|MouseEvents|RightMouseButton
  (params (Key :type Key%20Structure :default "None"))
  (:Pressed
    (Utilities|FlowControl|Delay 0.8)
    (|rightGrab)
    (|rightDrop)))

(event Input|KeyboardEvents|Q
  (params (Key :type Key%20Structure :default "None"))
  (bind _pickupbox (Variables|Default|GetpickUpBox))
  (:Pressed
    (Utilities|FlowControl|Delay 0.8)
    (if (Variables|Default|GetleftEquip)
      (for _array_element (Collision|GetOverlappingActors _pickupbox "/Game/Dynamic/Food/foodContainer_BP.foodContainer_BP_C" :!class /Script/Engine.PrimitiveComponent)
        (bind _asfood_container_bp (Utilities|Casting|CastTofoodContainer_BP _array_element))
        (bind _asplating_bp (Utilities|Casting|CastToplating_BP (Variables|Default|GetleftItem)))
        (Default|Fill _asplating_bp _asfood_container_bp))
      (else
        (for _array_element_2 (Collision|GetOverlappingActors _pickupbox "/Game/Dynamic/Food/foodContainer_BP.foodContainer_BP_C" :!class /Script/Engine.PrimitiveComponent)
          (bind _asfood_container_bp_2 (Utilities|Casting|CastTofoodContainer_BP _array_element_2))
          (Default|UnequipInteract _asfood_container_bp_2))))))

(event Input|KeyboardEvents|I
  (params (Key :type Key%20Structure :default "None"))
  (bind _returnvalue (Game|GetPlayerController 0))
  ;[1 1 1] Change Photos displayed
  (:Released
    (Utilities|Array|ForEachLoopwithBreak (Collision|GetOverlappingActors "/Game/Dynamic/Interfaces/Picture_BP.Picture_BP_C" :!class /Script/Engine.Actor) :!label _label
      (:LoopBody
        (if true
          (bind _returnvalue_2 (UserInterface|CreateWidget "/Game/Dynamic/System/GUI/PhotoChooser_BP.PhotoChooser_BP_C"))
          (UserInterface|Viewport|AddtoViewport _returnvalue_2 0)
          (Variables|/Script/Engine.PlayerController|SetbShowMouseCursor _returnvalue true)
          (Input|SetInputModeUIOnly _returnvalue _returnvalue_2 "DoNotLock" false)
          (goto _label Break))))))

(fn ConstructionScript)

(fn SubmitDish
  (params (Dish :type Dish%20Struc%20Structure)))